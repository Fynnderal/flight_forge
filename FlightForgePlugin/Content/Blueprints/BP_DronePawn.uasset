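; Drone pawn with animated propellers and a third-person viewer camera: mouse input orbits the view and the wheel zooms the spring arm.
; Every Tick calls RotatePropellers, which counter-rotates diagonal propeller pairs while PropellersRotate is true.
; A float curve drives spin-up until the time counter reaches the curve's max value, which then becomes the constant per-frame rotation.
; Clearing the flag stops rotation instantly and resets the counter, with no spin-down.
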(event `self.ReceiveBeginPlay`)

(event `self.ReceiveTick`
  (params (DeltaSeconds :type "Float (single-precision)"))
  (`self.RotatePropellers` DeltaSeconds))

(event `InputVectorAxis|Mouse2D`
  (params (AxisValue :type "Vector Structure"))
  ;[1 1 1] 360 viewer
  (`self.AddControllerYawInput` (* AxisValue_X -1.0))
  (`self.AddControllerPitchInput` (* AxisValue_Y -1.0)))

(event `InputAxisKey|MouseWheelAxis`
  (params (AxisValue :type "Float (single-precision)"))
  (bind _thirdpersoncameraspringarm (`self.ThirdPersonCameraSpringArm`))
  ;[1 1 1] Zoom viewer
  (set `SpringArmComponent.TargetArmLength` (+ (`SpringArmComponent.TargetArmLength` _thirdpersoncameraspringarm) (* AxisValue -13.0)) _thirdpersoncameraspringarm))

(fn `UserConstructionScript`)