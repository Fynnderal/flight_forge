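; BP_DronePawn_Light is a drone pawn with third-person camera controls.
; On BeginPlay it waits three seconds, then turns off physics simulation on its root mesh component.
; Mouse movement feeds inverted yaw and pitch into the controller, and the mouse wheel changes the camera spring arm length to zoom.
; The construction script and macro are empty.
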(event `self.ReceiveBeginPlay`
  (`KismetSystemLibrary.Delay` 3.0)
  (`PrimitiveComponent.SetSimulatePhysics` (`self.RootMeshComponent`) false))

(event `InputVectorAxis|Mouse2D`
  (params (AxisValue :type "Vector Structure"))
  (`self.AddControllerYawInput` (* AxisValue_X -1.0))
  (`self.AddControllerPitchInput` (* AxisValue_Y -1.0)))

(event `InputAxisKey|MouseWheelAxis`
  (params (AxisValue :type "Float (single-precision)"))
  (bind _thirdpersoncameraspringarm (`self.ThirdPersonCameraSpringArm`))
  (set `SpringArmComponent.TargetArmLength` (+ (`SpringArmComponent.TargetArmLength` _thirdpersoncameraspringarm) (* AxisValue -13.0)) _thirdpersoncameraspringarm))

(fn `UserConstructionScript`)