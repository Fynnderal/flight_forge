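; Game mode Blueprint that spawns a camera view switcher actor at world origin on BeginPlay.
; New players restart at a player start looked up using the current level name.
; An unconnected chain would spawn five drones with different meshes in a row from the player start.
; SetWeather and SetDaytime are empty stubs.
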(event `self.ReceiveBeginPlay`
  (`|SpawnActorFromClass` "/FlightForgePlugin/Blueprints/BP_ChangeCameraView.BP_ChangeCameraView_C" (`KismetMathLibrary.Conv_VectorToTransform` (0.0 0.0 0.0)) "Undefined" "MultiplyWithRoot" null null))

(event `self.HandleStartingNewPlayer`
  (params (NewPlayer :type "PlayerController Object Reference"))
  (bind _returnvalue (`GameplayStatics.GetCurrentLevelName` true))
  (`self.RestartPlayerAtPlayerStart` NewPlayer (`self.K2_FindPlayerStart` NewPlayer _returnvalue)))

(fn `SetDaytime`
  (params (hour :type Integer) (minute :type Integer))
  (returns (ReturnValue :type Boolean)))

(fn `SetWeather`
  (params (TypeId :type Integer))
  (returns (ReturnValue :type Boolean)))

(fn `UserConstructionScript`)